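; Shootable enemy actor with a health bar widget component that is handed a reference to the enemy on BeginPlay.
; Tick rotates the widget to face the player character.
; Head and Body hits from first-person projectiles each subtract the same fixed damage from Hp.
; When Hp equals exactly zero, the actor destroys itself and calls CallKillEnemy on the player character with a fixed value.
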(event `self.ReceiveBeginPlay`
  (bind _asenemy_hp_bar (cast `/Game/UI/EnemyHpBar` (`WidgetComponent.GetUserWidgetObject` (`self.Widget`))))
  (set `/Game/UI/EnemyHpBar.enemy` self _asenemy_hp_bar))

(event `self.ReceiveTick`
  (params (DeltaSeconds :type "Float (single-precision)"))
  (bind _widget (`self.Widget`))
  (`SceneComponent.K2_SetWorldRotation` _widget (`KismetMathLibrary.FindLookAtRotation` (`SceneComponent.K2_GetComponentLocation` _widget) (`self.K2_GetActorLocation` (`GameplayStatics.GetPlayerCharacter` 0))) false false))

(event `self.head.OnComponentHit`
  (params (HitComponent :type "PrimitiveComponent Object Reference") (OtherActor :type "Actor Object Reference") (OtherComp :type "PrimitiveComponent Object Reference") (NormalImpulse :type "Vector Structure") (Hit :type "HitResult Structure (by ref)"))
  (bind _hp (`self.hp`))
  (cast `/Game/FirstPerson/Blueprints/BP_FirstPersonProjectile` OtherActor)
  (set `self.hp` (- _hp 10.0))
  (if (== _hp 0.0)
    (`self.K2_DestroyActor`)
    (bind _asbp_first_person_character (cast `/Game/FirstPerson/Blueprints/BP_FirstPersonCharacter` (`GameplayStatics.GetPlayerCharacter` 0)))
    (`/Game/FirstPerson/Blueprints/BP_FirstPersonCharacter.KillEnemy` _asbp_first_person_character 100.0)))

(event `self.body.OnComponentHit`
  (params (HitComponent :type "PrimitiveComponent Object Reference") (OtherActor :type "Actor Object Reference") (OtherComp :type "PrimitiveComponent Object Reference") (NormalImpulse :type "Vector Structure") (Hit :type "HitResult Structure (by ref)"))
  (bind _hp (`self.hp`))
  (cast `/Game/FirstPerson/Blueprints/BP_FirstPersonProjectile` OtherActor)
  (set `self.hp` (- _hp 10.0))
  (if (== _hp 0.0)
    (`self.K2_DestroyActor`)
    (bind _asbp_first_person_character (cast `/Game/FirstPerson/Blueprints/BP_FirstPersonCharacter` (`GameplayStatics.GetPlayerCharacter` 0)))
    (`/Game/FirstPerson/Blueprints/BP_FirstPersonCharacter.KillEnemy` _asbp_first_person_character 100.0)))

(fn `UserConstructionScript`)